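; Trigger zone that turns a shooting mode on and off as the player pawn enters and leaves it.
; BeginPlay caches the starting transforms of the listed Objects.
; On entry it enables BPShoot's CanShoot, zeroes those static mesh actors' physics velocities, restores their transforms, blends the view to TargetCam's owner and shows the cursor.
; On exit it disables shooting, blends back to the pawn and hides the cursor.
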(event `self.ReceiveBeginPlay`
  (`self.EnableInput` (`GameplayStatics.GetPlayerController` 0))
  (for (_array_element _array_index) (`self.Objects`)
    (`KismetArrayLibrary.Array_Set` (`self.OldObjectTransform`) _array_index (`self.GetTransform` _array_element) true)))

(event `self.Trigger.OnComponentBeginOverlap`
  (params (OverlappedComponent :type "PrimitiveComponent Object Reference") (OtherActor :type "Actor Object Reference") (OtherComp :type "PrimitiveComponent Object Reference") (OtherBodyIndex :type Integer) (bFromSweep :type Boolean) (SweepResult :type "HitResult Structure (by ref)"))
  (if (== OtherActor (`GameplayStatics.GetPlayerPawn` 0))
    (set `/Game/Blueprints/BP_Shoot.canShoot` true (`self.BP_Shoot`))
    (for (_array_element _array_index) (`self.Objects`)
      (bind _asstatic_mesh_actor (cast `StaticMeshActor` _array_element))
      (bind _staticmeshcomponent (`StaticMeshActor.StaticMeshComponent` _asstatic_mesh_actor))
      (`PrimitiveComponent.SetPhysicsLinearVelocity` _staticmeshcomponent (0.0 0.0 0.0) false "None")
      (`PrimitiveComponent.SetPhysicsAngularVelocityInDegrees` _staticmeshcomponent (0.0 0.0 0.0) false "None")
      (`self.K2_SetActorTransform` _array_element (`|GetArrayItem` (`self.OldObjectTransform`) _array_index) false false))
    (`PlayerController.SetViewTargetWithBlend` (`GameplayStatics.GetPlayerController` 0) (`ActorComponent.GetOwner` (`self.TargetCam`)) 1.0 "VTBlend_EaseInOut" 2.0 false)
    (set `PlayerController.bShowMouseCursor` true (`GameplayStatics.GetPlayerController` 0))))

(event `self.Trigger.OnComponentEndOverlap`
  (params (OverlappedComponent :type "PrimitiveComponent Object Reference") (OtherActor :type "Actor Object Reference") (OtherComp :type "PrimitiveComponent Object Reference") (OtherBodyIndex :type Integer))
  (if (== OtherActor (`GameplayStatics.GetPlayerPawn` 0))
    (set `/Game/Blueprints/BP_Shoot.canShoot` false (`self.BP_Shoot`))
    (`PlayerController.SetViewTargetWithBlend` (`GameplayStatics.GetPlayerController` 0) (`GameplayStatics.GetPlayerPawn` 0) 1.0 "VTBlend_EaseInOut" 2.0 false)
    (set `PlayerController.bShowMouseCursor` false (`GameplayStatics.GetPlayerController` 0))))

(fn `UserConstructionScript`)