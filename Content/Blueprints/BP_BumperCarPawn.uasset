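; BP_BumperCarPawn is a drivable bumper car pawn that moves through physics forces.
; Enhanced Input drives it: move pushes the Cube along its forward vector, and turn applies an offset force at the Turner component to rotate it.
; Look input rotates the controller.
; Pressing E repossesses the stored player pawn and removes the bumper car mapping context.
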(event `EnhancedInput|/Game/ThirdPerson/Input/Actions/IA_Look`
  (params (ActionValue :type "Vector2D Structure") (ElapsedSeconds :type "Float (double-precision)") (TriggeredSeconds :type "Float (double-precision)") (InputAction :type "InputAction Object Reference" :default "/Game/ThirdPerson/Input/Actions/IA_Look.IA_Look"))
  (:`Triggered`
    (`self.AddControllerYawInput` ActionValue_X)
    (`self.AddControllerPitchInput` ActionValue_Y)))

(event `EnhancedInput|/Game/imc/IA_BumperCar_Move`
  (params (ActionValue :type "Float (double-precision)") (ElapsedSeconds :type "Float (double-precision)") (TriggeredSeconds :type "Float (double-precision)") (InputAction :type "InputAction Object Reference" :default "/Game/imc/IA_BumperCar_Move.IA_BumperCar_Move"))
  (:`Triggered`
    (`PrimitiveComponent.AddForce` (`self.Cube`) (* (* ActionValue 100000.0) (`SceneComponent.GetForwardVector` (`self.Cube`))) "None" false)))

(event `EnhancedInput|/Game/imc/IA_BumperCar_Turn`
  (params (ActionValue :type "Float (double-precision)") (ElapsedSeconds :type "Float (double-precision)") (TriggeredSeconds :type "Float (double-precision)") (InputAction :type "InputAction Object Reference" :default "/Game/imc/IA_BumperCar_Turn.IA_BumperCar_Turn"))
  (bind _turner (`self.Turner`))
  (:`Triggered`
    (`PrimitiveComponent.AddForceAtLocation` (`self.Cube`) (* (* ActionValue 50000.0 -1.0) (`SceneComponent.GetForwardVector` _turner)) (`SceneComponent.K2_GetComponentLocation` _turner) "None")))

(event `Key|E`
  (params (Key :type "Key Structure"))
  (:`Pressed`
    (`Controller.Possess` (`GameplayStatics.GetPlayerController` 0) (`self.pawnPlayer`))
    (message `EnhancedInputSubsystemInterface.RemoveMappingContext` (pcsubsystem `EnhancedInputLocalPlayerSubsystem` (`GameplayStatics.GetPlayerController` 0)) "/Game/imc/IMC_BumperCar.IMC_BumperCar" (struct))))

(fn `UserConstructionScript`)