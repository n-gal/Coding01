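; BP_Shoot fires a physics ball toward the point under the mouse cursor on left click, whenever CanShoot is true.
; It traces the Visibility channel along the deprojected cursor ray to find the target, then spawns a small BP_Ball at the camera location.
; The ball's Sphere is set to physics-only collision and receives an impulse along the clamped, unit-length direction to the hit, scaled by ShootSpeed.
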(event `Key|LeftMouseButton` :consume false
  (params (Key :type "Key Structure"))
  (bind (_worldlocation _worlddirection) (`PlayerController.DeprojectMousePositionToWorld` (`GameplayStatics.GetPlayerController` 0)))
  (:`Pressed`
    (if (`self.canShoot`)
      (bind _outhit (`KismetSystemLibrary.LineTraceSingle` _worldlocation (+ _worldlocation (* _worlddirection 900000000.0)) "TraceTypeQuery1"))
      (bind _returnvalue (`|SpawnActorFromClass` "/Game/Blueprints/BP_Ball.BP_Ball_C" (`KismetMathLibrary.MakeTransform` (`PlayerCameraManager.GetCameraLocation` (`GameplayStatics.GetPlayerCameraManager` 0)) (struct) (`KismetMathLibrary.Conv_DoubleToVector` (`KismetMathLibrary.RandomFloatInRange` 0.1 0.1))) "Undefined" "MultiplyWithRoot" null null))
      (bind _sphere (`/Game/Blueprints/BP_Ball.Sphere` _returnvalue))
      (`PrimitiveComponent.SetCollisionEnabled` _sphere "PhysicsOnly")
      (`PrimitiveComponent.AddImpulse` _sphere (* (`KismetMathLibrary.ClampVectorSize` (- (`.Location` (`GameplayStatics.BreakHitResult` _outhit)) (`SceneComponent.K2_GetComponentLocation` _sphere)) 0.0 1.0) (`self.ShootSpeed`)) "None" false))))